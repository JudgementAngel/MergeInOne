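; Playable hummingbird character Blueprint from a low-poly bird pack, built on a parent class and adding a hover mode.
; On BeginPlay it runs the parent logic, then sets the flying rotation rate.
; Holding Left Shift enables hover mode, lowering max fly speed and raising flight braking on CharacterMovement until release.
; The key is bound directly in the event graph, and the construction script only calls the parent.
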(event `self.ReceiveBeginPlay`
  (`parent.ReceiveBeginPlay`)
  (set `self.Rotation Rate Flying` 600.0))

(event `Key|LeftShift`
  (params (Key :type "Key Structure"))
  (bind _charactermovement (`self.CharacterMovement`))
  (bind _charactermovement_2 (`self.CharacterMovement`))
  ;[1 1 1] Hover Mode
  (:`Pressed`
    (set `self.HoverMode` true)
    (set `CharacterMovementComponent.MaxFlySpeed` 300.0 _charactermovement_2)
    (set `CharacterMovementComponent.BrakingDecelerationFlying` 1000.0 _charactermovement_2))
  (:`Released`
    (set `self.HoverMode` false)
    (set `CharacterMovementComponent.MaxFlySpeed` 600.0 _charactermovement)
    (set `CharacterMovementComponent.BrakingDecelerationFlying` 500.0 _charactermovement)))

(fn `UserConstructionScript`
  (`parent.UserConstructionScript`))