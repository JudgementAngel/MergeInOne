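; Flamingo bird Blueprint from the Low Poly Bird pack that extends a parent class and adjusts its camera height for flight.
; Each tick runs the parent logic, then plays a height timeline forward while IsFlying is true and reverses it otherwise.
; The timeline output drives the camera boom's relative Z, easing the view between grounded and flying heights.
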(event `self.ReceiveTick`
  (params (DeltaSeconds :type "Float (single-precision)"))
  (`parent.ReceiveTick` DeltaSeconds)
  (`self.Camera Boom Height Tick`))

(event `Camera Boom Height Tick`
  ;[1 1 1] Set Camera Height
  (if (`self.IsFlying`)
    (bind (_direction _value) (`Timeline|CameraBoom Height` :!label _label)
      (:`Update`
        (`SceneComponent.K2_SetRelativeLocation` (`self.CameraBoom`) (`KismetMathLibrary.MakeVector` 0.0 0.0 _value) false false)))
    (else
      (goto _label :!via `Reverse`))))

(fn `UserConstructionScript`
  (`parent.UserConstructionScript`))