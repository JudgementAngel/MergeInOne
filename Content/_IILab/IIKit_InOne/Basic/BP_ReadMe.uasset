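; BP_ReadMe is an in-level notice for the InOne kit that shows version or date info and an optional missing-dependency warning as 3D text.
; The Construction Script picks the text from the SwitchInfo and Warning flags, styling it through a helper that sets materials and scale.
; The EventGraph holds only unconnected reference nodes, some commented with required or optional content packs and setup notes for vehicles, weather, damage UI, flight and birds.
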(fn `IIF_SetText3D`
  (params (InTextCom :type "Text3DComponent Object Reference") (InMaterial :type "MaterialInterface Object Reference") (InScale :type "Float (double-precision)"))
  (set `Text3DComponent.FrontMaterial` InMaterial InTextCom)
  (set `Text3DComponent.BevelMaterial` InMaterial InTextCom)
  (set `Text3DComponent.ExtrudeMaterial` InMaterial InTextCom)
  (set `Text3DComponent.BackMaterial` InMaterial InTextCom)
  (`SceneComponent.SetWorldScale3D` InTextCom (* InScale 1.0)))

(fn `UserConstructionScript`
  (bind _text3dcomponent (`self.Text3DComponent`))
  (bind _text3dcompwarning (`self.Text3DCompWarning`))
  (`|ExecutionSequence`
    (:`then_0`
      (`self.IIF_SetText3D` _text3dcomponent (`self.MI_Cyan`) 2.0)
      (if (`self.SwitchInfo`)
        (set `Text3DComponent.Text` "InOneTest \nCreation Date: 2024.10.9 \nPublish Date: 2024.11.25" _text3dcomponent)
        (else
          (set `Text3DComponent.Text` "InOneTest \nCurrent Version v1.3.1 \n2024.12.2" _text3dcomponent))))
    (:`then_1`
      (if (`self.Warning`)
        (`self.IIF_SetText3D` _text3dcompwarning (`self.MI_Red`) 1.5)
        (set `Text3DComponent.Text` "You must add Superhero Flight Animations and Ultra Dynamic Sky" _text3dcompwarning)))))